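; GA_jump is a Gameplay Ability that makes the avatar character jump.
; On activation it launches the character upward with a slight forward push, overriding vertical velocity while adding to horizontal velocity.
; It then commits the ability cost, applies the GE_jump_increment effect to itself, and ends.
; The cost is committed after the launch with its result unchecked, and a failed Character cast stops only the launch branch.
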(event Ability|EventActivateAbility
  (bind _returnvalue (Ability|GetAvatarActorfromActorInfo))
  (bind _returnvalue_2 (Transformation|GetActorForwardVector _returnvalue))
  (bind _returnvalue_3 (* _returnvalue_2 6e+01))
  (bind (_x _y) (Math|Vector|BreakVector _returnvalue_3))
  (Utilities|FlowControl|Sequence
    (:then_0
      (bind _ascharacter (Utilities|Casting|CastToCharacter _returnvalue))
      (Character|LaunchCharacter _ascharacter (Math|Vector|MakeVectorNetQuantize _x _y 6e+02) false true))
    (:then_1
      (Ability|CommitAbilityCost false))
    (:then_2
      (GameplayEffects|ApplyGameplayEffectToSelf :self (Ability|GetAbilitySystemComponentfromActorInfo) :GameplayEffectClass "/Game/base/ability_system/effects/jump/GE_jump_increment.GE_jump_increment_C"))
    (:then_3
      (Ability|EndAbility))))