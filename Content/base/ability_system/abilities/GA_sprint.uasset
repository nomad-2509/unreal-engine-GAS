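; Sprint gameplay ability that raises the avatar's max walk speed, applies GE_sprint, commits cost and plays a sprint montage when tagged as sprinting.
; Fast looping timers cancel it when forward velocity is too low or cost is unaffordable.
; An end-sprint gameplay event or montage interruption also cancels it.
; Ending lowers speed, stops the montage task and clears timers; GE_sprint removal nodes are left unconnected.
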(event Custom|check_sprint_cost
  (bind _returnvalue (Class|GameplayAbility|CheckAbilityCost))
  (if (not _returnvalue)
    (Ability|CancelAbility)))

(event Custom|check_for_run
  (bind _returnvalue (Ability|GetAvatarActorfromActorInfo))
  (if (<= (Math|Vector|DotProduct (Transformation|GetVelocity _returnvalue) (Transformation|GetActorForwardVector _returnvalue)) 2.5e+02)
    (Ability|CancelAbility)))

(event Ability|EventActivateAbility
  (Utilities|FlowControl|Sequence
    (:then_0
      (CallFunction|CheckforRun)
      (bind _returnvalue (Utilities|Time|SetTimerbyEvent (delegate Custom|check_for_run) 0.02 true))
      (Variables|Default|Settimer_check_for_run _returnvalue))
    (:then_1
      (CallFunction|CheckSprintCost)
      (bind _returnvalue_2 (Utilities|Time|SetTimerbyEvent (delegate Custom|check_sprint_cost) 0.02 true))
      (Variables|Default|Settimer_check_cost _returnvalue_2))
    (:then_2
      (bind _ascharacter (Utilities|Casting|CastToCharacter (Ability|GetAvatarActorfromActorInfo)))
      (Variables|/Script/Engine.CharacterMovementComponent|SetMaxWalkSpeed (Variables|/Script/Engine.Character|GetCharacterMovement _ascharacter) (+ (Class|MovementComponent|GetMaxSpeed (Variables|/Script/Engine.Character|GetCharacterMovement _ascharacter)) 1e+03)))
    (:then_3
      (bind _returnvalue_3 (GameplayEffects|ApplyGameplayEffectToSelf :self (Ability|GetAbilitySystemComponentfromActorInfo) :GameplayEffectClass "/Game/base/ability_system/effects/sprint/GE_sprint.GE_sprint_C"))
      (Variables|Default|Seteffect_sprint_mov_speed _returnvalue_3))
    (:then_4
      (Ability|CommitAbilityCost false))
    (:then_5
      ;[0 0 0] DEBUG - must check if sprinting
      (if (GameplayTags|HasMatchingGameplayTag (Ability|GetAbilitySystemComponentfromActorInfo) "(TagName=\"movement.sprint\")")
        (bind _asynctaskproxy (|PlayMontageandWaitProxy "None" "/Game/base/assets/animations/sprint/TravelMode_Sprint_Montage.TravelMode_Sprint_Montage" 1.0 "None" true 1.0 0.0)
          (:then
            (Variables|Default|Settask_sprint_anim _asynctaskproxy))
          (:OnInterrupted
            (Ability|CancelAbility :!label _label))
          (:OnCancelled
            (goto _label)))))
    (:then_6
      (bind _asynctaskproxy_2 (Ability|Tasks|WaitGameplayEvent "(TagName=\"movement.sprint.end\")" 0)
        (:then
          (Variables|Default|Settask_sprint_end _asynctaskproxy_2))
        (:EventReceived
          (Ability|CancelAbility))))))

(event Ability|EventOnEndAbility
  (params (bWasCancelled :type Boolean))
  (bind _task_sprint_anim (Variables|Default|Gettask_sprint_anim))
  (Utilities|FlowControl|Sequence
    (:then_0
      (bind _ascharacter (Utilities|Casting|CastToCharacter (Ability|GetAvatarActorfromActorInfo)))
      (Variables|/Script/Engine.CharacterMovementComponent|SetMaxWalkSpeed (Variables|/Script/Engine.Character|GetCharacterMovement _ascharacter) (+ (Class|MovementComponent|GetMaxSpeed (Variables|/Script/Engine.Character|GetCharacterMovement _ascharacter)) -1e+03)))
    (:then_1
      (Utilities|IsValid _task_sprint_anim
        (:Is%20Valid
          (GameplayTasks|EndTask _task_sprint_anim))))
    (:then_2)
    (:then_3)
    (:then_4
      (Utilities|Time|ClearandInvalidateTimerbyHandle (Variables|Default|Gettimer_check_for_run))
      (Utilities|Time|ClearandInvalidateTimerbyHandle (Variables|Default|Gettimer_check_cost)))))