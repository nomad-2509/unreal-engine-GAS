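; GA_lina_buff is a gameplay ability for Lina, triggered by a gameplay event, that grants her a steal-stack buff.
; It switches on the event tag, then checks the event target's ability system for parry and perfect-dodge tags.
; It cancels only if the target has both tags; otherwise it applies GE_lina_buff_steal_stack to the owner and ends.
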(event Ability|EventActivateAbilityFromEvent
  (params (EventData :type Gameplay%20Event%20Data%20Structure%20%28by%20ref%29))
  (bind (_eventtag _instigator _target) (Utilities|Struct|BreakGameplayEventData EventData))
  (|SwitchGameplayTag _eventtag
    (:combat.range.hit
      (if (not (and (GameplayTags|HasMatchingGameplayTag (Ability|GetAbilitySystemComponent _target) "(TagName=\"combat.block.parry\")") (GameplayTags|HasMatchingGameplayTag (Ability|GetAbilitySystemComponent _target) "(TagName=\"combat.dodge.perfect\")")))
        (GameplayEffects|ApplyGameplayEffectToSelf :self (Ability|GetAbilitySystemComponentfromActorInfo) :GameplayEffectClass "/Game/base/ability_system/effects/lina/GE_lina_buff_steal_stack.GE_lina_buff_steal_stack_C" :Level 0.0)
        (Ability|EndAbility)
        (else
          (Ability|CancelAbility))))))