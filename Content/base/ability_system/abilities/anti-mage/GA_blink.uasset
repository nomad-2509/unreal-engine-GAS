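; Anti-mage Gameplay Ability that blinks the avatar to a camera-aimed point within range.
; The targeting event loops a local debug-capsule preview of the destination, found by a camera-forward capsule trace extended by camera-to-player distance.
; The confirm event passes that point through a target-data task, fires the blink GameplayCue and commits.
; After a delay, the authority moves the avatar if the range check passes, then ends the ability.
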(event Custom|event_blink_to_location
  (if (CallFunction|ValidateBlinkRange)
    (Transformation|SetActorLocation (Ability|GetAvatarActorfromActorInfo) (Variables|Default|Getblink_location) false false)
    (Ability|EndAbility)
    (else
      (Ability|EndAbility))))

(event Ability|EventActivateAbilityFromEvent
  (params (EventData :type Gameplay%20Event%20Data%20Structure%20%28by%20ref%29))
  (|SwitchGameplayTag (.EventTag (Utilities|Struct|BreakGameplayEventData EventData))
    (:ability.target.targetting
      (Pawn|IsLocallyControlled
        (:True
          (CallFunction|ShowBlinkLocation)
          (bind _returnvalue (Utilities|Time|SetTimerbyFunctionName 0 "show_blink_location" 0.02 true))
          (Variables|Default|Setblink_targetting_timer _returnvalue))))
    (:ability.target.confirm
      (Utilities|Time|ClearandInvalidateTimerbyHandle (Variables|Default|Getblink_targetting_timer))
      (Utilities|FlowControl|Sequence
        (:then_0
          (bind _blink_location (CallFunction|MakeBlinkTargetLocation))
          (Variables|Default|Setblink_location _blink_location))
        (:then_1
          (bind (_asynctaskproxy _datahandle) (|CreateTargetData (Variables|Default|Getblink_location) 0 false false)
            (:then
              (Variables|Default|Settask_target_data _asynctaskproxy))
            (:target_data
              (Variables|Default|Setblink_location (.Location (Collision|BreakHitResult (Ability|TargetData|GetHitResultfromTargetData _datahandle))))
              (Utilities|FlowControl|Sequence
                (:then_0
                  (Class|GameplayAbility|AddGameplayCuewithParams "(TagName=\"GameplayCue.blink\")" (Ability|GameplayCue|MakeGameplayCueParameters :Location (Variables|Default|Getblink_location)) true)
                  (Class|GameplayAbility|ExecuteGameplayCuewithParams "(TagName=\"GameplayCue.blink\")" (Ability|GameplayCue|MakeGameplayCueParameters :Location (Variables|Default|Getblink_location))))
                (:then_1
                  (Ability|HasAuthority
                    (:True
                      (Utilities|Time|SetTimerbyEvent (delegate Custom|event_blink_to_location) (Variables|Default|Getblink_delay)))))
                (:then_2
                  (Ability|CommitAbility))))))))))

(event Ability|EventOnEndAbility
  (params (bWasCancelled :type Boolean))
  (bind _task_target_data (Variables|Default|Gettask_target_data))
  (bind _task_blink_confirm (Variables|Default|Gettask_blink_confirm))
  (Utilities|FlowControl|Sequence
    (:then_0
      (Utilities|IsValid _task_target_data
        (:Is%20Valid
          (GameplayTasks|EndTask _task_target_data))))
    (:then_1
      (Utilities|IsValid _task_blink_confirm
        (:Is%20Valid
          (GameplayTasks|EndTask _task_blink_confirm))))))

(fn MakeBlinkTargetLocation
  (bind _returnvalue (Game|GetPlayerCameraManager 0))
  (bind _transformcomponent (Variables|/Script/Engine.PlayerCameraManager|GetTransformComponent _returnvalue))
  (bind _returnvalue_2 (Transformation|GetWorldLocation _transformcomponent))
  (Utilities|FlowControl|Sequence
    (:then_0
      (LocalVariables|Setblink_start_location_ _returnvalue_2)
      (LocalVariables|Setblink_end_location_ (+ _returnvalue_2 (* (Math|Vector|GetForwardVector _transformcomponent) (+ (Variables|Default|Getblink_range) (CallFunction|GetCameraDistancefromPlayer))))))
    (:then_1
      (bind (_outhit _returnvalue_3) (Collision|CapsuleTraceByChannel (LocalVariables|Getblink_start_location_) (LocalVariables|Getblink_end_location_) 3e+01 8e+01 "TraceTypeQuery2" false (Utilities|Array|MakeArray (Ability|GetAvatarActorfromActorInfo)) "None" true "(R=1.000000,G=0.000000,B=0.000000,A=1.000000)" "(R=0.000000,G=1.000000,B=0.000000,A=1.000000)" 2.0))
      (if _returnvalue_3
        (LocalVariables|Setblink_end_location_ (.Location (Collision|BreakHitResult _outhit)))))
    (:then_2
      (return (LocalVariables|Getblink_end_location_)))))

(fn GetCameraDistancefromPlayer
  (bind _returnvalue (Ability|GetAvatarActorfromActorInfo))
  (bind _returnvalue_2 (Game|GetPlayerCameraManager 0))
  (bind _returnvalue_3 (Transformation|GetActorLocation _returnvalue))
  (bind _transformcomponent (Variables|/Script/Engine.PlayerCameraManager|GetTransformComponent _returnvalue_2))
  (bind _returnvalue_4 (Transformation|GetWorldLocation _transformcomponent))
  (bind (_x _y) (Class|KismetMathLibrary|BreakVector3f _returnvalue_3))
  (bind (_x_2 _y_2) (Math|Vector|BreakVector _returnvalue_4))
  (return (Math|Vector|Distance(Vector) (Math|Vector|MakeVector _x_2 _y_2 0.0) (Math|Vector|MakeVector _x _y 0.0))))

(fn ShowBlinkLocation
  (Utilities|FlowControl|Sequence
    (:then_0
      (LocalVariables|Setblink_target_start_location (Transformation|GetWorldLocation (Variables|/Script/Engine.PlayerCameraManager|GetTransformComponent (Game|GetPlayerCameraManager 0))))
      (bind _blink_location (CallFunction|MakeBlinkTargetLocation))
      (LocalVariables|Setblink_end_location _blink_location))
    (:then_2
      (Rendering|Debug|DrawDebugCapsule (LocalVariables|Getblink_end_location) 8e+01 3e+01 "0, 0, 0" "(R=0.000000,G=1.000000,B=0.785954,A=1.000000)" 0.1 1e+01))))

(fn ValidateBlinkRange
  (return (<= (Math|Vector|Distance(Vector) (Variables|Default|Getblink_location) (Transformation|GetActorLocation (Ability|GetAvatarActorfromActorInfo))) (+ (Variables|Default|Getblink_range) 3e+01))))