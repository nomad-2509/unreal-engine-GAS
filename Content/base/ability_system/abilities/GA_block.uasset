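; Gameplay ability that makes the avatar block and opens a parry window.
; On activation it looks up its montage by ability class in the HERO row of DT_animations, plays it and applies GE_parry_window to itself.
; A Combat.block.end gameplay event ends the ability, while an interrupted or cancelled montage cancels it.
; The parry window effect is removed by handle whenever the ability ends.
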(event Ability|EventActivateAbility
  (Utilities|IsValid (Ability|GetAvatarActorfromActorInfo)
    (:Is%20Valid
      (Utilities|FlowControl|Sequence
        (:then_0
          (bind _returnvalue (Utilities|GetDataTableRow "/Game/base/model/DT_animations.DT_animations" "HERO")
            (:then
              (if (.ReturnValue (Utilities|Map|Find (Utilities|Struct|Breakanimation_data _returnvalue) (Utilities|GetClass self)))
                (Variables|Default|Setblock_anim_montage (Utilities|Array|Get(acopy) (Utilities|Struct|Breakanim_montage_array (.Value (Utilities|Map|Find (Utilities|Struct|Breakanimation_data _returnvalue) (Utilities|GetClass self))))))
                (else
                  (Ability|CancelAbility))))))
        (:then_1
          (bind _asynctaskproxy (|PlayMontageandWaitProxy "None" (Variables|Default|Getblock_anim_montage) 1.0 "None" true 1.0 0.0)
            (:then
              (Variables|Default|Setblock_animation_task _asynctaskproxy))
            (:OnInterrupted
              (Ability|CancelAbility :!label _label))
            (:OnCancelled
              (goto _label))))
        (:then_2
          (bind _returnvalue_2 (GameplayEffects|ApplyGameplayEffectToSelf :self (Ability|GetAbilitySystemComponentfromActorInfo) :GameplayEffectClass "/Game/base/ability_system/effects/block/GE_parry_window.GE_parry_window_C"))
          (Variables|Default|Setparry_window_effect_handle _returnvalue_2))
        (:then_3
          (bind _asynctaskproxy_2 (Ability|Tasks|WaitGameplayEvent "(TagName=\"combat.block.end\")" 0)
            (:then
              (Variables|Default|Setblock_end_task _asynctaskproxy_2))
            (:EventReceived
              (Ability|EndAbility))))))
    (:Is%20Not%20Valid
      (Ability|CancelAbility))))

(event Ability|EventOnEndAbility
  (params (bWasCancelled :type Boolean))
  (Ability|RemoveGameplayEffectFromOwnerWithHandle (Variables|Default|Getparry_window_effect_handle)))