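; GA_ranged is a Gameplay Ability that plays a cycling series of animation montages for the avatar.
; It looks up the avatar's class name in DT_animations, then picks the montage array keyed by this ability's class, cancelling if either is missing.
; Each activation advances a wrapping index, with a retriggerable three-second delay after ending to reset the sequence.
; Montage completion or blend-out ends the ability, while interruption cancels it.
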(event Ability|EventActivateAbility
  (Utilities|FlowControl|Sequence
    (:then_0
      (bind _returnvalue (Utilities|GetDataTableRow "/Game/base/model/DT_animations.DT_animations" (Utilities|String|StringToName (Utilities|GetClassDisplayName (Utilities|GetClass (Ability|GetAvatarActorfromActorInfo)))))
        (:then
          (if (.ReturnValue (Utilities|Map|Find (Utilities|Struct|Breakanimation_data _returnvalue) (Utilities|GetClass self)))
            (Variables|Default|Setcurrent_montage_array (Utilities|Struct|Breakanim_montage_array (.Value (Utilities|Map|Find (Utilities|Struct|Breakanimation_data _returnvalue) (Utilities|GetClass self)))))
            (else
              (Ability|CancelAbility))))
        (:RowNotFound
          (Ability|CancelAbility))))
    (:then_1
      (bind _output_get (Variables|Default|Setcurrent_montage_array_length (Utilities|Array|Length (Variables|Default|Getcurrent_montage_array))))
      (Variables|Default|Setmontage_index (Math|Integer|%(Integer) (Variables|Default|Getmontage_index) _output_get)))
    (:then_2
      (bind _asynctaskproxy (|PlayMontageandWaitProxy "None" (Utilities|Array|Get(acopy) (Variables|Default|Getcurrent_montage_array) (Variables|Default|Getmontage_index)) 1.0 "None" true 1.0 0.0)
        (:then
          (Variables|Default|Settask_melee_montage _asynctaskproxy))
        (:OnCompleted
          (Ability|EndAbility :!label _label))
        (:OnBlendOut
          (goto _label))
        (:OnInterrupted
          (Ability|CancelAbility :!label _label_2))
        (:OnCancelled
          (goto _label_2))))
    (:then_3
      (Math|Integer|IncrementInt (Variables|Default|Getmontage_index)))))

(event Ability|EventOnEndAbility
  (params (bWasCancelled :type Boolean))
  (Utilities|FlowControl|Sequence
    (:then_0
      (Utilities|FlowControl|RetriggerableDelay 3.0)
      (Variables|Default|Setmontage_index 0))))