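; Gameplay Ability for dashing, triggered by event and branching on its tag into dodge or sprint.
; Dodge applies a short root-motion force along player input (backward if none) or fixed world -X for non-players, plus GE_dodge_increment.
; Sprint manually raises walk speed, applies GE_sprint and plays a montage from DT_animations' HERO row.
; A Movement.dash.end event lowers speed, removes the sprint effect and ends the ability.
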(event Ability|EventActivateAbilityFromEvent
  (params (EventData :type Gameplay%20Event%20Data%20Structure%20%28by%20ref%29))
  (Utilities|FlowControl|Sequence
    (:then_0
      (bind _asynctaskproxy (Ability|Tasks|WaitGameplayEvent "(TagName=\"movement.dash.end\")" 0)
        (:then
          (Variables|Default|Settask_sprint_end _asynctaskproxy))
        (:EventReceived
          (Utilities|FlowControl|Sequence
            (:then_0
              ;[0 0 0] Remove Movement Speed Effect. For now, resetting movement speed manually
              (bind _ascharacter (Utilities|Casting|CastToCharacter (Ability|GetAvatarActorfromActorInfo)))
              (Variables|/Script/Engine.CharacterMovementComponent|SetMaxWalkSpeed (Variables|/Script/Engine.Character|GetCharacterMovement _ascharacter) (+ (Class|MovementComponent|GetMaxSpeed (Variables|/Script/Engine.Character|GetCharacterMovement _ascharacter)) -1e+03)))
            (:then_1
              (Ability|RemoveGameplayEffectFromOwnerWithHandle (Variables|Default|Geteffect_sprint_mov_speed)))
            (:then_2
              (Ability|EndAbility))))))
    (:then_1
      (|SwitchGameplayTag (.EventTag (Utilities|Struct|BreakGameplayEventData EventData))
        (:combat.dodge
          ;[0.4 0.2 0 0.5] Dodge
          (Utilities|FlowControl|Sequence
            (:then_0
              (bind _ascharacter_2 (Utilities|Casting|CastToCharacter (Ability|GetAvatarActorfromActorInfo)))
              (if (Pawn|IsPlayerControlled _ascharacter_2)
                (Variables|Default|Setdodge_direction (CallFunction|GetDodgeVectorfromPlayerInput))
                (else
                  (Variables|Default|Setdodge_direction (CallFunction|MakeDodgeTargetData)))))
            (:then_1
              (bind _asynctaskproxy_2 (Ability|Tasks|ApplyRootMotionConstantForce "None" (Variables|Default|Getdodge_direction) 1.5e+03 0.1 false 0 "ClampVelocity" "0, 0, 0" 3e+02)
                (:then
                  (Variables|Default|Settask_dodge _asynctaskproxy_2))
                (:OnFinish
                  (Ability|EndAbility))))
            (:then_2
              (Ability|CommitAbility))
            (:then_3
              (GameplayEffects|ApplyGameplayEffectToSelf :self (Ability|GetAbilitySystemComponentfromActorInfo) :GameplayEffectClass "/Game/base/ability_system/effects/dodge/GE_dodge_increment.GE_dodge_increment_C"))))
        (:movement.sprint
          ;[0 0.4 0.2 0.5] Sprint
          (Utilities|FlowControl|Sequence
            (:then_0
              ;;[0 0 0] Modify movement speed using a Gameplay Effect
              ;; (For now, modifying walk speed manually)
              (bind _ascharacter_3 (Utilities|Casting|CastToCharacter (Ability|GetAvatarActorfromActorInfo)))
              (Variables|/Script/Engine.CharacterMovementComponent|SetMaxWalkSpeed (Variables|/Script/Engine.Character|GetCharacterMovement _ascharacter_3) (+ (Class|MovementComponent|GetMaxSpeed (Variables|/Script/Engine.Character|GetCharacterMovement _ascharacter_3)) 1e+03)))
            (:then_1
              (bind _returnvalue (GameplayEffects|ApplyGameplayEffectToSelf :self (Ability|GetAbilitySystemComponentfromActorInfo) :GameplayEffectClass "/Game/base/ability_system/effects/sprint/GE_sprint.GE_sprint_C"))
              (Variables|Default|Seteffect_sprint_mov_speed _returnvalue))
            (:then_2
              (Ability|CommitAbilityCost false))
            (:then_3
              (bind _returnvalue_2 (Utilities|GetDataTableRow "/Game/base/model/DT_animations.DT_animations" "HERO")
                (:then
                  (if (.ReturnValue (Utilities|Map|Find (Utilities|Struct|Breakanimation_data _returnvalue_2) (Utilities|GetClass self)))
                    (Variables|Default|Setsprint_anim_montage (Utilities|Array|Get(acopy) (Utilities|Struct|Breakanim_montage_array (.Value (Utilities|Map|Find (Utilities|Struct|Breakanimation_data _returnvalue_2) (Utilities|GetClass self))))))
                    (else
                      (Ability|CancelAbility))))))
            (:then_4
              (bind _asynctaskproxy_3 (|PlayMontageandWaitProxy "None" (Variables|Default|Getsprint_anim_montage) 1.0 "None" true 1.0 0.0)
                (:then
                  (Variables|Default|Settask_sprint_anim _asynctaskproxy_3))
                (:OnInterrupted
                  (Ability|CancelAbility :!label _label))
                (:OnCancelled
                  (goto _label))))))))))

(fn GetDodgeVectorfromPlayerInput
  (bind _returnvalue (Ability|GetAvatarActorfromActorInfo))
  (bind _asbase_player_controller (Utilities|Casting|CastTobase_player_controller (Game|GetPlayerController 0)))
  (LocalVariables|Setx_ (Class|BasePlayerController|GetMovementX _asbase_player_controller))
  (LocalVariables|Sety_ (Class|BasePlayerController|GetMovementY _asbase_player_controller))
  (Utilities|FlowControl|Sequence
    (:then_0
      (if (and (Math|Float|NearlyEqual(Float) (Class|BasePlayerController|GetMovementX _asbase_player_controller) 0.0 0.01) (Math|Float|NearlyEqual(Float) (Class|BasePlayerController|GetMovementY _asbase_player_controller) 0.0 0.01))
        (LocalVariables|Setx_ -1.0)
        (LocalVariables|Sety_ 0.0)))
    (:then_1
      (return (Math|Vector|Normalize (+ (* (Transformation|GetActorForwardVector _returnvalue) (LocalVariables|Getx_)) (* (Transformation|GetActorRightVector _returnvalue) (LocalVariables|Gety_))))))))

(fn MakeDodgeTargetData
  (return "-1.000000,0.000000,0.000000"))