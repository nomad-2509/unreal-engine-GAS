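; BP_MINION is a minion pawn with melee combat and a world-space attribute widget.
; Melee begin and end events forward to CombatComponent.
; Two seconds after BeginPlay it activates its block ability through the Ability System, if one is registered, then initializes widgets and HUD.
; Each tick the widget turns toward the player camera, enlarges at medium range for readability and hides beyond a cutoff distance.
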(event EventBeginPlay
  (bind _initial_ability_container (Variables|Default|Getinitial_ability_container))
  (bind (_value _returnvalue) (Utilities|Map|Find _initial_ability_container "(TagName=\"combat.block\")"))
  (|CallParentFunction)
  (Utilities|FlowControl|Delay 2.0)
  (Utilities|FlowControl|Sequence
    (:then_0
      (if _returnvalue
        (Abilities|TryActivateAbilitybyClass (Ability|GetAbilitySystemComponent self) _value true)))
    (:then_1
      (Class|BASECHAR|InitializeWidgets)
      (Class|BASECHAR|InitializeHUD))))

(event EventMeleeEnd
  ;[0.5 0 0.1 0.5] MELEE
  (Default|MeleeEnd (Variables|Default|Getcombat_component)))

(event EventTick
  (params (DeltaSeconds :type Float%20%28single-precision%29))
  (CallFunction|BaseAttributeWidgetRender))

(event EventMeleeBegin
  ;[0.5 0 0.1 0.5] MELEE
  (Default|MeleeBegin (Variables|Default|Getcombat_component)))

(fn ConstructionScript)

(fn BaseAttributeWidgetRender
  (bind _returnvalue (Game|GetPlayerCameraManager 0))
  (bind _widget_base_attributes (Variables|Default|Getwidget_base_attributes))
  (Utilities|IsValid (Variables|Default|Getwidget_base_attributes)
    (:Is%20Valid
      (Utilities|IsValid _returnvalue
        (:Is%20Valid
          (LocalVariables|Setcamera _returnvalue)
          (Utilities|FlowControl|Sequence
            (:then_0
              (Transformation|SetWorldRotation (Variables|Default|Getwidget_base_attributes) (Math|Rotator|FindLookatRotation (Transformation|GetActorLocation) (Transformation|GetWorldLocation (Variables|/Script/Engine.PlayerCameraManager|GetTransformComponent (LocalVariables|Getcamera)))) false false))
            (:then_1
              (Utilities|FlowControl|Sequence
                (:then_0
                  (if (>= (Math|Vector|Distance(Vector) (Transformation|GetActorLocation) (Transformation|GetWorldLocation (Variables|/Script/Engine.PlayerCameraManager|GetTransformComponent (LocalVariables|Getcamera)))) (LocalVariables|Getwidget_hide_distance))
                    (Development|SetHiddeninGame (Variables|Default|Getwidget_base_attributes) true false)
                    (else
                      (Development|SetHiddeninGame (Variables|Default|Getwidget_base_attributes) false false)
                      (if (>= (Math|Vector|Distance(Vector) (Transformation|GetActorLocation) (Transformation|GetWorldLocation (Variables|/Script/Engine.PlayerCameraManager|GetTransformComponent (LocalVariables|Getcamera)))) (LocalVariables|Getwidget_medium_distance))
                        (Transformation|SetWorldScale3D _widget_base_attributes "0.330000,0.330000,0.330000")
                        (else
                          (Transformation|SetWorldScale3D _widget_base_attributes "0.200000,0.200000,0.200000"))))))))))))))

(fn GetCombatComponent
  (return (Variables|Default|Getcombat_component)))