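; BP_HERO is the hero pawn Blueprint, acting as a thin melee layer over its CombatComponent.
; MeleeBegin and MeleeEnd events forward the start and end of an attack to that component.
; Overlaps on left and right hand and leg colliders pass the other actor straight to PerformMelee, with no filtering in the hero.
; A GetCombatComponent function exposes the component to callers.
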(event OnComponentBeginOverlap(hand_r)
  (params (OverlappedComponent :type Primitive%20Component%20Object%20Reference) (OtherActor :type Actor%20Object%20Reference) (OtherComp :type Primitive%20Component%20Object%20Reference) (OtherBodyIndex :type Integer) (bFromSweep :type Boolean) (SweepResult :type Hit%20Result%20Structure%20%28by%20ref%29))
  ;[0.5 0 0.1 0.5] MELEE
  (Default|PerformMelee (Variables|Default|Getcombat_component) OtherActor))

(event OnComponentBeginOverlap(hand_l)
  (params (OverlappedComponent :type Primitive%20Component%20Object%20Reference) (OtherActor :type Actor%20Object%20Reference) (OtherComp :type Primitive%20Component%20Object%20Reference) (OtherBodyIndex :type Integer) (bFromSweep :type Boolean) (SweepResult :type Hit%20Result%20Structure%20%28by%20ref%29))
  ;[0.5 0 0.1 0.5] MELEE
  (Default|PerformMelee (Variables|Default|Getcombat_component) OtherActor))

(event OnComponentBeginOverlap(leg_l)
  (params (OverlappedComponent :type Primitive%20Component%20Object%20Reference) (OtherActor :type Actor%20Object%20Reference) (OtherComp :type Primitive%20Component%20Object%20Reference) (OtherBodyIndex :type Integer) (bFromSweep :type Boolean) (SweepResult :type Hit%20Result%20Structure%20%28by%20ref%29))
  ;[0.5 0 0.1 0.5] MELEE
  (Default|PerformMelee (Variables|Default|Getcombat_component) OtherActor))

(event OnComponentBeginOverlap(leg_r)
  (params (OverlappedComponent :type Primitive%20Component%20Object%20Reference) (OtherActor :type Actor%20Object%20Reference) (OtherComp :type Primitive%20Component%20Object%20Reference) (OtherBodyIndex :type Integer) (bFromSweep :type Boolean) (SweepResult :type Hit%20Result%20Structure%20%28by%20ref%29))
  ;[0.5 0 0.1 0.5] MELEE
  (Default|PerformMelee (Variables|Default|Getcombat_component) OtherActor))

(event EventMeleeBegin
  ;[0.5 0 0.1 0.5] MELEE
  (Default|MeleeBegin (Variables|Default|Getcombat_component)))

(event EventMeleeEnd
  ;[0.5 0 0.1 0.5] MELEE
  (Class|IFCombat|MeleeEnd(Message) (Variables|Default|Getcombat_component)))

(fn ConstructionScript)

(fn GetCombatComponent
  (return (Variables|Default|Getcombat_component)))