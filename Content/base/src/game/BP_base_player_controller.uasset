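; Base player controller that maps hard-coded debug keys to Gameplay Ability System actions on the controlled BASE_CHAR.
; Most keys look up an ability class by gameplay tag in the pawn's InitialAbilityContainer and activate it, while sprint and block releases send end events.
; Held melee retries on a fast looping timer, and C sends a dodge event, then sprint if held long enough.
; F prints minion attribute values.
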(event Custom|sprint_activate
  ;[0 0.5 0.1 0.5] MOVEMENT
  (Ability|SendGameplayEventtoActor (Pawn|GetControlledPawn) "(TagName=\"movement.sprint\")"))

(event Custom|triggered_melee
  ;[0.5 0 0.1 0.5] COMBAT
  (if (Variables|Default|Getmelee_held)
    (bind _asbase_char (Utilities|Casting|CastToBASE_CHAR (Pawn|GetControlledPawn)))
    (if (.ReturnValue (Utilities|Map|Find (Variables|/Script/GAS_tutorial.BASE_CHAR|Getinitial_ability_container _asbase_char) "(TagName=\"combat.melee\")"))
      (Abilities|TryActivateAbilitybyClass (Ability|GetAbilitySystemComponent _asbase_char) (.Value (Utilities|Map|Find (Variables|/Script/GAS_tutorial.BASE_CHAR|Getinitial_ability_container _asbase_char) "(TagName=\"combat.melee\")")) true))
    (else
      (Utilities|Time|ClearandInvalidateTimerbyHandle (Variables|Default|Getmelee_held_timer)))))

(event EventBeginPlay)

(event EventTick
  (params (DeltaSeconds :type Float%20%28single-precision%29)))

(event Input|KeyboardEvents|DebugKeyQ
  (params (Key :type Key%20Structure :default "None") (ActionValue :type Input%20Action%20Value%20Structure))
  ;[0 0.1 0.5 0.5] ABILITIES
  (:Pressed
    (bind _asbase_char (Utilities|Casting|CastToBASE_CHAR (Pawn|GetControlledPawn)))
    (if (.ReturnValue (Utilities|Map|Find (Variables|/Script/GAS_tutorial.BASE_CHAR|Getinitial_ability_container _asbase_char) "(TagName=\"ability.slot.1\")"))
      (Abilities|TryActivateAbilitybyClass (Ability|GetAbilitySystemComponent _asbase_char) (.Value (Utilities|Map|Find (Variables|/Script/GAS_tutorial.BASE_CHAR|Getinitial_ability_container _asbase_char) "(TagName=\"ability.slot.1\")")) true))))

(event Input|KeyboardEvents|DebugKeyF
  (params (Key :type Key%20Structure :default "None") (ActionValue :type Input%20Action%20Value%20Structure))
  (:Pressed
    (bind _outactors (Actor|GetAllActorsOfClass "/Game/base/pawn/BP_MINION.BP_MINION_C"))
    (bind _array_element (Utilities|Array|ForEachLoopwithBreak _outactors)
      (:LoopBody
        (Utilities|FlowControl|Sequence
          (:then_0
            (Development|PrintString (Utilities|String|Append "MINION health: " (Utilities|String|ToString(Float) (.ReturnValue (Ability|Attribute|GetFloatAttributefromAbilitySystemComponent (Ability|GetAbilitySystemComponent _array_element) "(AttributeName=\"health\",Attribute=/Script/GAS_tutorial.BASE_attribute_set:health,AttributeOwner=/Script/CoreUObject.Class'\"/Script/GAS_tutorial.BASE_attribute_set\"')")))) true true "(R=0.500000,G=0.000000,B=0.000000,A=1.000000)" 3.0))
          (:then_1
            (Development|PrintString (Utilities|String|Append "MINION mana: " (Utilities|String|ToString(Float) (.ReturnValue (Ability|Attribute|GetFloatAttributefromAbilitySystemComponent (Ability|GetAbilitySystemComponent _array_element) "(AttributeName=\"mana\",Attribute=/Script/GAS_tutorial.BASE_attribute_set:mana,AttributeOwner=/Script/CoreUObject.Class'\"/Script/GAS_tutorial.BASE_attribute_set\"')")))) true true "(R=0.000000,G=0.100000,B=0.500000,A=1.000000)" 3.0))
          (:then_2
            (Development|PrintString (Utilities|String|Append "MINION stamina: " (Utilities|String|ToString(Float) (.ReturnValue (Ability|Attribute|GetFloatAttributefromAbilitySystemComponent (Ability|GetAbilitySystemComponent _array_element) "(AttributeName=\"stamina\",Attribute=/Script/GAS_tutorial.BASE_attribute_set:stamina,AttributeOwner=/Script/CoreUObject.Class'\"/Script/GAS_tutorial.BASE_attribute_set\"')")))) true true "(R=0.000000,G=0.500000,B=0.000000,A=1.000000)" 3.0)))))))

(event Input|KeyboardEvents|DebugKeyC
  (params (Key :type Key%20Structure :default "None") (ActionValue :type Input%20Action%20Value%20Structure))
  ;[0 0.5 0.1 0.5] MOVEMENT
  (:Pressed
    (Ability|SendGameplayEventtoActor (Pawn|GetControlledPawn) "(TagName=\"combat.dodge\")")
    (bind _returnvalue (Utilities|Time|SetTimerbyEvent (delegate Custom|sprint_activate) 3.0))
    (Variables|Default|Setsprint_held_timer _returnvalue))
  (:Released
    (Utilities|Time|ClearandInvalidateTimerbyHandle (Variables|Default|Getsprint_held_timer))
    (Ability|SendGameplayEventtoActor (Pawn|GetControlledPawn) "(TagName=\"movement.dash.end\")")))

(event Input|KeyboardEvents|DebugKeyX
  (params (Key :type Key%20Structure :default "None") (ActionValue :type Input%20Action%20Value%20Structure))
  ;[0 0.5 0.1 0.5] MOVEMENT
  (:Pressed
    (bind _asbase_char (Utilities|Casting|CastToBASE_CHAR (Pawn|GetControlledPawn)))
    (if (.ReturnValue (Utilities|Map|Find (Variables|/Script/GAS_tutorial.BASE_CHAR|Getinitial_ability_container _asbase_char) "(TagName=\"movement.sprint\")"))
      (Abilities|TryActivateAbilitybyClass (Ability|GetAbilitySystemComponent _asbase_char) (.Value (Utilities|Map|Find (Variables|/Script/GAS_tutorial.BASE_CHAR|Getinitial_ability_container _asbase_char) "(TagName=\"movement.sprint\")")) true)))
  (:Released
    (Ability|SendGameplayEventtoActor (Pawn|GetControlledPawn) "(TagName=\"movement.sprint.end\")")))

(event Input|KeyboardEvents|DebugKeyZ
  (params (Key :type Key%20Structure :default "None") (ActionValue :type Input%20Action%20Value%20Structure))
  ;[0 0.5 0.1 0.5] MOVEMENT
  (:Pressed
    (bind _asbase_char (Utilities|Casting|CastToBASE_CHAR (Pawn|GetControlledPawn)))
    (if (.ReturnValue (Utilities|Map|Find (Variables|/Script/GAS_tutorial.BASE_CHAR|Getinitial_ability_container _asbase_char) "(TagName=\"combat.dodge\")"))
      (Abilities|TryActivateAbilitybyClass (Ability|GetAbilitySystemComponent _asbase_char) (.Value (Utilities|Map|Find (Variables|/Script/GAS_tutorial.BASE_CHAR|Getinitial_ability_container _asbase_char) "(TagName=\"combat.dodge\")")) true))))

(event Input|MouseEvents|DebugKeyLeftMouseButton
  (params (Key :type Key%20Structure :default "None") (ActionValue :type Input%20Action%20Value%20Structure))
  ;[0.5 0 0.1 0.5] COMBAT
  (:Pressed
    (Variables|Default|Setmelee_held true)
    (bind _returnvalue (Utilities|Time|SetTimerbyEvent (delegate Custom|triggered_melee) 0.02 true))
    (Variables|Default|Setmelee_held_timer _returnvalue))
  (:Released
    (Variables|Default|Setmelee_held false)))

(event Input|MouseEvents|DebugKeyRightMouseButton
  (params (Key :type Key%20Structure :default "None") (ActionValue :type Input%20Action%20Value%20Structure))
  ;[0.5 0 0.1 0.5] COMBAT
  (:Pressed
    (bind _asbase_char (Utilities|Casting|CastToBASE_CHAR (Pawn|GetControlledPawn)))
    (if (.ReturnValue (Utilities|Map|Find (Variables|/Script/GAS_tutorial.BASE_CHAR|Getinitial_ability_container _asbase_char) "(TagName=\"combat.block\")"))
      (Abilities|TryActivateAbilitybyClass (Ability|GetAbilitySystemComponent _asbase_char) (.Value (Utilities|Map|Find (Variables|/Script/GAS_tutorial.BASE_CHAR|Getinitial_ability_container _asbase_char) "(TagName=\"combat.block\")")) true)))
  (:Released
    (Ability|SendGameplayEventtoActor (Pawn|GetControlledPawn) "(TagName=\"combat.block.end\")")))

(event Input|KeyboardEvents|DebugKeySpaceBar
  (params (Key :type Key%20Structure :default "None") (ActionValue :type Input%20Action%20Value%20Structure))
  ;[0 0.5 0.1 0.5] MOVEMENT
  (:Pressed
    (bind _asbase_char (Utilities|Casting|CastToBASE_CHAR (Pawn|GetControlledPawn)))
    (if (.ReturnValue (Utilities|Map|Find (Variables|/Script/GAS_tutorial.BASE_CHAR|Getinitial_ability_container _asbase_char) "(TagName=\"movement.jump\")"))
      (Abilities|TryActivateAbilitybyClass (Ability|GetAbilitySystemComponent _asbase_char) (.Value (Utilities|Map|Find (Variables|/Script/GAS_tutorial.BASE_CHAR|Getinitial_ability_container _asbase_char) "(TagName=\"movement.jump\")")) true))))

(fn ConstructionScript)